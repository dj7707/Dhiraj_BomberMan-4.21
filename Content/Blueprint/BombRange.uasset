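; BombRange is a pickup Blueprint that increases a player's bomb range when collected.
; When an actor overlaps its Box, it checks whether the class is Player_1 or Player_2 and adds a fixed amount to that player's bomb range stored in NewGameInstance.
; The pickup then destroys itself, and other overlapping actors are ignored.
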(event `self.Box.OnComponentBeginOverlap`
  (params (OverlappedComponent :type "PrimitiveComponent Object Reference") (OtherActor :type "Actor Object Reference") (OtherComp :type "PrimitiveComponent Object Reference") (OtherBodyIndex :type Integer) (bFromSweep :type Boolean) (SweepResult :type "HitResult Structure (by ref)"))
  (bind _returnvalue (`GameplayStatics.GetObjectClass` OtherActor))
  (bind _returnvalue_2 (`GameplayStatics.GetGameInstance`))
  (if (== _returnvalue "/Game/Blueprint/Player_1.Player_1_C")
    (bind _asnew_game_instance (cast `/Game/Blueprints/NewGameInstance` _returnvalue_2))
    (set `/Game/Blueprints/NewGameInstance.Player_1BombRange` (+ (`/Game/Blueprints/NewGameInstance.Player_1BombRange` _asnew_game_instance) 25.0) _asnew_game_instance)
    (`self.K2_DestroyActor` :!label _label)
    (elif (== _returnvalue "/Game/Blueprint/Player_2.Player_2_C")
      (bind _asnew_game_instance_2 (cast `/Game/Blueprints/NewGameInstance` _returnvalue_2))
      (set `/Game/Blueprints/NewGameInstance.Player_2BombRange` (+ (`/Game/Blueprints/NewGameInstance.Player_2BombRange` _asnew_game_instance_2) 25.0) _asnew_game_instance_2)
      (goto _label))))

(fn `UserConstructionScript`)
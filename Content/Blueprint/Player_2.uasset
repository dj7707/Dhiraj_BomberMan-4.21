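; Player 2's Blueprint, a physics-driven cube that moves and drops bombs.
; Every tick it pushes the cube with a mass-independent force from Player 2's forward/back and right/left inputs, scaled by a speed variable.
; Pressing Enter spawns a Bomb_2 above the cube and increments the bomb count, unless that count equals the maximum.
; Nothing in these graphs decrements the count.
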(event `self.ReceiveTick`
  (params (DeltaSeconds :type "Float (single-precision)"))
  (bind _player_2speed (`self.Player_2Speed`))
  ;[1 1 1] Player2 Movement
  (`PrimitiveComponent.AddForce` (`self.Cube`) (`KismetMathLibrary.MakeVector` (* (`self.GetInputAxisValue`) _player_2speed) (* (`self.GetInputAxisValue`) _player_2speed)) "None" true))

(event `Key|Enter`
  (params (Key :type "Key Structure"))
  (:`Pressed`
    (if (!= (`self.Bombs`) (`self.Bombs_Max`))
      (`|SpawnActorFromClass` "/Game/Blueprint/Bomb_2.Bomb_2_C" (`KismetMathLibrary.Conv_VectorToTransform` (`KismetMathLibrary.MakeVector` (.x (`SceneComponent.K2_GetComponentLocation` (`self.Cube`))) (.y (`SceneComponent.K2_GetComponentLocation` (`self.Cube`))) (+ (.z (`SceneComponent.K2_GetComponentLocation` (`self.Cube`))) 250.0))) "Undefined" "OverrideRootScale" null null)
      (`/Engine/EditorBlueprintResources/StandardMacros.IncrementInt` (`self.Bombs`)))))

(fn `UserConstructionScript`)
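; WallBreak is a breakable wall Blueprint that can drop a random power-up at its Cube's location.
; ChanceDrop runs cascading random checks to spawn a BombBooster, BombRange, PlayerSpeed or PlayerHealthBoost, or nothing if all fail.
; Each comparison makes its own roll, and the speed and health checks share the same thresholds, so later items depend on earlier checks failing.
; The file contains no caller for ChanceDrop and no destruction logic.
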(fn `ChanceDrop`
  (bind _returnvalue (`KismetMathLibrary.RandomFloatInRange` 0.0 80.0))
  (bind _returnvalue_2 (`KismetMathLibrary.Conv_VectorToTransform` (`SceneComponent.K2_GetComponentLocation` (`self.Cube`))))
  ;[1 1 1] wall Break
  (if (< _returnvalue 20.0)
    (`|SpawnActorFromClass` "/Game/Blueprint/BombBooster.BombBooster_C" _returnvalue_2 "Undefined" "OverrideRootScale" null null)
    (elif (> _returnvalue 70.0)
      (`|SpawnActorFromClass` "/Game/Blueprint/BombRange.BombRange_C" _returnvalue_2 "Undefined" "OverrideRootScale" null null)
      (elif (and (< _returnvalue 70.0) (> _returnvalue 40.0))
        (`|SpawnActorFromClass` "/Game/Blueprint/PlayerSpeed.PlayerSpeed_C" _returnvalue_2 "Undefined" "OverrideRootScale" null null)
        (elif (and (< _returnvalue 70.0) (> _returnvalue 40.0))
          (`|SpawnActorFromClass` "/Game/Blueprint/PlayerHealthBoost.PlayerHealthBoost_C" _returnvalue_2 "Undefined" "OverrideRootScale" null null))))))

(fn `UserConstructionScript`)
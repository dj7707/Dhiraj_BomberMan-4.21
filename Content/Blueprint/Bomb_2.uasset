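; Player 2's timed bomb, which damages players and breaks walls in its blast range.
; On BeginPlay it sizes its overlap sphere from the GameInstance, then steps material and light intensity through a two-second fuse.
; It then decrements Player_2's bomb count and checks overlaps, updating HP and scores and triggering wall drops before destroying itself.
; Either player hit destroys the first loop's Player_2 element, not the overlapped actor.
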(event `self.ReceiveBeginPlay`
  (bind _gameinstance (`self.GameInstance`))
  (bind _gameinstance_2 (`self.GameInstance`))
  (bind _gameinstance_3 (`self.GameInstance`))
  (bind _pointlight (`self.PointLight`))
  ;[1 1 1] Bomb And wall break
  (bind _asnew_game_instance (cast `/Game/Blueprints/NewGameInstance` (`GameplayStatics.GetGameInstance`)))
  (set `self.GameInstance` _asnew_game_instance)
  (`SphereComponent.SetSphereRadius` (`self.Spher Coll`) (`/Game/Blueprints/NewGameInstance.Player_2BombRange` (`self.GameInstance`)) true)
  (`PrimitiveComponent.SetMaterial` (`self.Sphere`) 0 "/Game/MATs/Bomb1_MAT.Bomb1_MAT")
  (`KismetSystemLibrary.Delay` 0.5)
  (`LightComponent.SetIntensity` _pointlight 3000.0)
  (`PrimitiveComponent.SetMaterial` (`self.Sphere`) 0 "/Game/MATs/Bomb1_MAT_2.Bomb1_MAT_2")
  (`KismetSystemLibrary.Delay` 0.5)
  (`LightComponent.SetIntensity` _pointlight 6000.0)
  (`PrimitiveComponent.SetMaterial` (`self.Sphere`) 0 "/Game/MATs/Bomb1_MAT_3.Bomb1_MAT_3")
  (`KismetSystemLibrary.Delay` 0.5)
  (`LightComponent.SetIntensity` _pointlight 9000.0)
  (`PrimitiveComponent.SetMaterial` (`self.Sphere`) 0 "/Game/MATs/Bomb1_MAT_4.Bomb1_MAT_4")
  (`KismetSystemLibrary.Delay` 0.5)
  (bind _outactors (`GameplayStatics.GetAllActorsOfClass` "/Game/Blueprint/Player_2.Player_2_C"))
  (for _array_element _outactors
    (`/Engine/EditorBlueprintResources/StandardMacros.DecrementInt` (`/Game/Blueprint/Player_2.Bombs` _array_element)))
  (bind _output_get (set `self.Overlap` (`PrimitiveComponent.GetOverlappingActors` (`self.Spher Coll`) null)))
  (for _array_element_2 _output_get
    (bind _returnvalue (`GameplayStatics.GetObjectClass` _array_element_2))
    ;;[1 1 1] player2 Scoring
    (if (== _returnvalue "/Game/Blueprint/Player_2.Player_2_C")
      (set `/Game/Blueprints/NewGameInstance.Player_2 Score` (- (`/Game/Blueprints/NewGameInstance.Player_2 Score` _gameinstance_3) 50.0) _gameinstance_3)
      (`/Engine/EditorBlueprintResources/StandardMacros.DecrementInt` (`/Game/Blueprints/NewGameInstance.Player_2HP` _gameinstance_3)
        (:`  `
          (`self.K2_DestroyActor` _array_element :!label _label)))
      (elif (== _returnvalue "/Game/Blueprint/Player_1.Player_1_C")
        (set `/Game/Blueprints/NewGameInstance.Player_2 Score` (+ (`/Game/Blueprints/NewGameInstance.Player_2 Score` _gameinstance_2) 80.0) _gameinstance_2)
        (set `/Game/Blueprints/NewGameInstance.Player_1 Score` (- (`/Game/Blueprints/NewGameInstance.Player_1 Score` _gameinstance_2) 80.0) _gameinstance_2)
        (`/Engine/EditorBlueprintResources/StandardMacros.DecrementInt` (`/Game/Blueprints/NewGameInstance.Player_1HP` _gameinstance_2)
          (:`  `
            (goto _label)))
        (elif (== _returnvalue "/Game/Blueprint/WallBreak.WallBreak_C")
          (bind _aswall_break (cast `/Game/Blueprint/WallBreak` _array_element_2))
          (`/Game/Blueprint/WallBreak.ChanceDrop` _aswall_break)
          (set `/Game/Blueprints/NewGameInstance.Player_2 Score` (+ (`/Game/Blueprints/NewGameInstance.Player_2 Score` _gameinstance) 10.0) _gameinstance)
          (`self.K2_DestroyActor` _array_element_2)))))
  (`self.K2_DestroyActor`))

(fn `UserConstructionScript`)
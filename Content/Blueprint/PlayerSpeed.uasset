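; PlayerSpeed is a pickup actor that gives a speed boost to whichever of the two players touches it.
; When an actor begins overlapping its Box, it compares that actor's class to Player_1 and Player_2, then casts to the matching one.
; It adds a fixed amount to that player's own speed variable and destroys itself, with no logic to revert the boost.
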(event `self.Box.OnComponentBeginOverlap`
  (params (OverlappedComponent :type "PrimitiveComponent Object Reference") (OtherActor :type "Actor Object Reference") (OtherComp :type "PrimitiveComponent Object Reference") (OtherBodyIndex :type Integer) (bFromSweep :type Boolean) (SweepResult :type "HitResult Structure (by ref)"))
  (bind _returnvalue (`GameplayStatics.GetObjectClass` OtherActor))
  (if (== _returnvalue "/Game/Blueprint/Player_1.Player_1_C")
    (bind _asplayer_1 (cast `/Game/Blueprint/Player_1` OtherActor))
    (set `/Game/Blueprint/Player_1.Player_1Speed` (+ (`/Game/Blueprint/Player_1.Player_1Speed` _asplayer_1) 350.0) _asplayer_1)
    (`self.K2_DestroyActor` :!label _label)
    (elif (== _returnvalue "/Game/Blueprint/Player_2.Player_2_C")
      (bind _asplayer_2 (cast `/Game/Blueprint/Player_2` OtherActor))
      (set `/Game/Blueprint/Player_2.Player_2Speed` (+ (`/Game/Blueprint/Player_2.Player_2Speed` _asplayer_2) 350.0) _asplayer_2)
      (goto _label))))

(fn `UserConstructionScript`)